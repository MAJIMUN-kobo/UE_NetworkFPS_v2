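; Gameplay game mode that picks each player's pawn class and tracks the coin total.
; GetDefaultPawnClassForController looks up the player's name in the game instance's selected-character map, falling back to BP_Player when no valid class is found.
; AddCoin adds to TotalPoint on BP_OurGameInstance and returns the new total.
; KillPlayer is an empty stub, and the TotalPoint reset in the event graph is unconnected.
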(event EventBeginPlay)

(event EventTick
  (params (DeltaSeconds :type Float%20%28single-precision%29)))

(fn ConstructionScript)

(fn GetDefaultPawnClassforController
  (params (InController :type Controller%20Object%20Reference))
  (bind _returnvalue (Game|GetGameInstance))
  (bind _playerstate (Variables|/Script/Engine.Controller|GetPlayerState InController))
  (bind _returnvalue_2 (PlayerState|GetPlayerName _playerstate))
  (bind _asbp_our_game_instance (Utilities|Casting|CastToBP_OurGameInstance _returnvalue))
  (bind _selectedcharactersofallplayers (Variables|/Game/Lobby/BP_OurGameInstance.BP_OurGameInstance_C|GetSelectedCharactersOfAllPlayers _asbp_our_game_instance))
  (bind _value (Utilities|Map|Find _selectedcharactersofallplayers _returnvalue_2))
  (if (Utilities|IsValidClass _value)
    (return _value)
    (else
      (return "/Game/BP_Player/BP_Player.BP_Player_C"))))

(fn AddCoin
  (params (B :type Integer))
  (bind _asbp_our_game_instance (Utilities|Casting|CastToBP_OurGameInstance (Game|GetGameInstance)))
  (bind _output_get (Variables|/Game/Lobby/BP_OurGameInstance.BP_OurGameInstance_C|SetTotalPoint _asbp_our_game_instance (+ (Variables|/Game/Lobby/BP_OurGameInstance.BP_OurGameInstance_C|GetTotalPoint _asbp_our_game_instance) B)))
  (return _output_get))

(fn KillPlayer)