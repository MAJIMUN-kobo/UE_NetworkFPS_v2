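; Gameplay GameState that tracks death counts for the red and blue teams and shows them on screen.
; BeginPlay creates a DeathPointUI widget and adds it to the viewport.
; AddDeathCount increments the red or blue count by TeamID and prints a debug string.
; Tick casts the stored widget and copies both counts into it every frame.
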(event EventBeginPlay
  (bind _returnvalue (UserInterface|CreateWidget "/Game/Lobby/DeathPointUI.DeathPointUI_C"))
  (bind _output_get (Variables|Default|SetDeathPointUI _returnvalue))
  (UserInterface|Viewport|AddtoViewport _output_get 0))

(event EventTick
  (params (DeltaSeconds :type Float%20%28single-precision%29))
  (bind _asdeath_point_ui (Utilities|Casting|CastToDeathPointUI (Variables|Default|GetDeathPointUI)))
  (Variables|/Game/Lobby/DeathPointUI.DeathPointUI_C|SetDeathPointBlue _asdeath_point_ui (Variables|Default|GetDeathCount_blue))
  (Variables|/Game/Lobby/DeathPointUI.DeathPointUI_C|SetDeathPointRed _asdeath_point_ui (Variables|Default|GetDeathCount_red)))

(fn ConstructionScript)

(fn AddDeathCount
  (params (TeamID :type Integer))
  (switch int TeamID
    (:0
      (bind _result (Math|Integer|IncrementInt (Variables|Default|GetDeathCount_red))
        (:%20%20
          (Variables|Default|SetDeathCount_red _result)
          (Development|PrintString "redDeath"))))
    (:1
      (bind _result_2 (Math|Integer|IncrementInt (Variables|Default|GetDeathCount_blue))
        (:%20%20
          (Variables|Default|SetDeathCount_blue _result_2)
          (Development|PrintString "blueDeath"))))))