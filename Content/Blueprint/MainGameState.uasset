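; Main game state Blueprint that tracks team IDs and death counts for Red and Blue teams.
; SetTeamID writes a lobby player controller's TeamID into the TeamIDs array, which BeginPlay seeds with one entry.
; AddDeathCount increments the matching team's counter, with debug prints.
; The timer is unfinished, as Tick only zeroes TimerSeconds while active, and the death-point widget creation is disconnected.
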(event EventBeginPlay
  (Utilities|Array|Add (Variables|Default|GetTeamIDs) 0))

(event EventTick
  (params (DeltaSeconds :type Float%20%28single-precision%29))
  (if (Variables|Default|GetIsTimerActive)
    (Variables|Default|SetTimerSeconds 0.0)))

(fn ConstructionScript)

(fn SetTeamID
  (params (PCs :type Player%20Controller%20Object%20Reference))
  (bind _asbp_lobby_pc (Utilities|Casting|CastToBP_LobbyPC PCs))
  (Utilities|Array|SetArrayElem (Variables|Default|GetTeamIDs) 0 (Variables|/Game/Lobby/BP_LobbyPC.BP_LobbyPC_C|GetTeamID _asbp_lobby_pc))
  (Development|PrintString (Utilities|String|ToString(Text) (Utilities|Text|FormatText "登録ID={id}" 0)) true true "(R=0.000000,G=0.660000,B=1.000000,A=1.000000)" 1e+01))

(fn AddDeathCount
  (params (TeamID :type Integer))
  (switch int TeamID
    (:0
      (bind _result (Math|Integer|IncrementInt (Variables|Default|GetDeathCount_red))
        (:%20%20
          (Variables|Default|SetDeathCount_red _result)
          (Development|PrintString "redDeath"))))
    (:1
      (bind _result_2 (Math|Integer|IncrementInt (Variables|Default|GetDeathCount_blue))
        (:%20%20
          (Variables|Default|SetDeathCount_blue _result_2)
          (Development|PrintString "blueDeath"))))))