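; BP_EnemyAI is an enemy Blueprint that handles taking damage and dying, with no AI behavior in its graphs.
; Point damage calls DamageValueSync, which spawns a DamageActor at the hit location, subtracts Health, prints it and destroys the enemy at zero or below.
; BeginPlay caches the EnemyHelthBar from the Widget component so each hit can update its health value.
; The HelthBarOnServer and HelthBarSync events are empty stubs.
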(event Custom|HelthBarOnServer)

(event Custom|HelthBarSync)

(event Custom|DamageValueSync
  (params (CastDamage :type Float%20%28double-precision%29))
  (Game|SpawnActorfromClass "/Game/DamegeUi/DamageActor.DamageActor_C" (Math|Transform|MakeTransform (stale Game|Damage|EventPointDamage HitLocation) "0, 0, 0" "1.000000,1.000000,1.000000") "Undefined" "MultiplyWithRoot" 0 CastDamage 0)
  (bind _output_get (Variables|Default|SetHealth (- (Variables|Default|GetHealth) CastDamage)))
  (Development|PrintString (Utilities|String|ToString(Float) _output_get))
  (Variables|/Game/Animation/EnemyHelthBar.EnemyHelthBar_C|SetEnemyWidgetHelth (Variables|Default|GetAs%20Enemy%20Helth%20Bar) _output_get)
  (if (<= (Variables|Default|GetHealth) 0.0)
    (Development|PrintString "Dead")
    (Actor|DestroyActor)))

(event EventBeginPlay
  (bind _asenemy_helth_bar (Utilities|Casting|CastToEnemyHelthBar (UserInterface|GetUserWidgetObject (Variables|Default|GetWidget))))
  (Variables|Default|SetAs%20Enemy%20Helth%20Bar _asenemy_helth_bar))

(event Game|Damage|EventPointDamage
  (params (Damage :type Float%20%28single-precision%29) (DamageType :type Damage%20Type%20Object%20Reference) (HitLocation :type Vector :default "0, 0, 0") (HitNormal :type Vector :default "0, 0, 0") (HitComponent :type Primitive%20Component%20Object%20Reference) (BoneName :type Name :default "None") (ShotFromDirection :type Vector :default "0, 0, 0") (InstigatedBy :type Controller%20Object%20Reference) (DamageCauser :type Actor%20Object%20Reference) (HitInfo :type Hit%20Result%20Structure%20%28by%20ref%29))
  (CallFunction|DamageValueSync Damage))

(fn ConstructionScript)