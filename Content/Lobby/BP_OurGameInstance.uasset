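; Game instance that handles multiplayer session hosting and invites, and holds player team and point state.
; CreateSession creates an Advanced Sessions session, then opens the Lobby level as a listen server.
; An accepted invite destroys any current session and joins the invited one whether or not the destroy succeeds.
; Initialize resets TotalPoint to its class default, while setter and getter functions expose the player's team ID.
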(event Custom|CreateSession
  (|AdvancedSession 0 (Game|GetPlayerController 0) 100 0 false true false true true true false false false true false true
    (:OnSuccess
      (Game|OpenLevel(byObjectReference) "/Game/Map/Lobby.Lobby" true "listen"))))

(event Custom|Event%20On%20Session%20Invite%20Accepted
  (params (SearchResult :type Blueprint%20Session%20Result%20Structure%20%28by%20ref%29))
  (|DestroySession (Game|GetPlayerController 0)
    (:OnSuccess
      _)
    (:OnFailure
      _))
  (|JoinSession (Game|GetPlayerController 0) SearchResult))

(fn Initialize
  (Variables|Default|SetTotalPoint (.TotalPoint (Utilities|GetClassDefaults "BP_OurGameInstance_C"))))

(fn SetTeamID
  (params (teamId :type Integer))
  (Variables|Default|SetplayerTeamId teamId))

(fn GetTeamID
  (return (Variables|Default|GetplayerTeamId)))