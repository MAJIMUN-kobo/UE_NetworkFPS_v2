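; Lobby platform actor that stands for one numbered player slot, with a button widget meant to open a friend list.
; SpawnCharacter stores the player controller, has BP_LobbyGM select character class index 0 and hides the button.
; Character clearing, server-only friend list setup and show/hide logic exist but are disconnected: Clear, BeginPlay and ShowFriendList are empty, and SetUpServer is only called from unwired nodes.
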(event Custom|SpawnCharacter
  (params (PC :type Player%20Controller%20Object%20Reference))
  (Variables|Default|SetPC PC)
  (Development|PrintString (Utilities|String|ToString(Text) (Utilities|Text|FormatText "土台番号 = { number }" (Variables|Default|GetPlatformNumber))) true true "(R=0.000000,G=0.660000,B=1.000000,A=1.000000)" 1e+01)
  (Default|SelectCharacterClassbyIndex (.AsBP%20Lobby%20GM (Utilities|Casting|CastToBP_LobbyGM (Game|GetGameMode))) (Variables|Default|GetPC))
  (Rendering|SetVisibility (Variables|Default|GetOpenFriendListButton) false false))

(event Custom|Clear
  ;[1 1 1] player削除処理
)

(event EventBeginPlay)

(fn ConstructionScript)

(fn ShowFriendList
  (params (bShow :type Boolean)))

(fn SetUpServer
  (if (Networking|IsServer)
    (bind _returnvalue (Actor|GetActorOfClass "/Game/Lobby/BP_FriendList.BP_FriendList_C"))
    (Variables|Default|SetFriendListRef _returnvalue)
    (bind _aswb_open_friend_list_button (Utilities|Casting|CastToWB_OpenFriendListButton (UserInterface|GetWidget (Variables|Default|GetOpenFriendListButton))))
    (Variables|/Game/Lobby/Widget/WB_OpenFriendListButton.WB_OpenFriendListButton_C|SetLobbyPlayerPlatformRef _aswb_open_friend_list_button self)
    (Rendering|SetVisibility (Variables|Default|GetOpenFriendListButton) true false)))