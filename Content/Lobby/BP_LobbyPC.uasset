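; Lobby player controller that manages a player's name, ready state, and character and team choice before a match.
; BeginPlay creates the gameplay widget, submits the GameInstance's player name, ends in game-only input and caches the HUD's lobby UI.
; Name changes and R-key ready toggles (blocked during countdown) update a lobby info struct pushed to BP_LobbyGM.
; A looping MultiGate cycles character classes and stores TeamID in the GameInstance; countdown UI calls are unwired.
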(event Custom|TryAgainUpdatingLobbyInfo
  (Utilities|FlowControl|Delay 0.1)
  (bind _asbp_lobby_gm (Utilities|Casting|CastToBP_LobbyGM (Game|GetGameMode)))
  (Default|UpdatePlayerLobbyInfo _asbp_lobby_gm self))

(event Custom|SetPlayerNameOnServer
  (params (PlayerName :type Text))
  ;[1 1 1] Comment
  (Utilities|Struct|SetmembersinS_PlayerLobbyInfo (Variables|Default|GetPlayerLobbyInfoPC) PlayerName)
  (bind _asbp_lobby_gm (Utilities|Casting|CastToBP_LobbyGM (Game|GetGameMode)))
  (Default|UpdatePlayerLobbyInfo _asbp_lobby_gm self))

(event Custom|ToggleReadyStatusOnServer
  (bind _playerlobbyinfopc (Variables|Default|GetPlayerLobbyInfoPC))
  (if (not (Variables|/Game/Lobby/BP_LobbyGM.BP_LobbyGM_C|GetStartMatchCountdownActive (.AsBP%20Lobby%20GM (Utilities|Casting|CastToBP_LobbyGM (Game|GetGameMode)))))
    (Utilities|Struct|SetmembersinS_PlayerLobbyInfo _playerlobbyinfopc (not (.bReady (Utilities|Struct|BreakS_PlayerLobbyInfo _playerlobbyinfopc))))
    (bind _asbp_lobby_gm (Utilities|Casting|CastToBP_LobbyGM (Game|GetGameMode)))
    (Default|UpdatePlayerLobbyInfo _asbp_lobby_gm self)
    (Development|PrintString "foge")))

(event Custom|OnStartMatch
  (Input|DisableInput self))

(event Custom|StartMatchCountdown
  (params (bStart :type Boolean))
  (if bStart
    _))

(event Custom|SelectCharacterOnServer
  (Utilities|FlowControl|MultiGate false true 1
    (:Out%200
      (Variables|Default|SetTeamID 0)
      (Default|SelectCharacterClassbyIndex (Variables|Default|GetLobbyGM_Ref) self))
    (:Out%201
      (Variables|Default|SetTeamID 1)
      (Default|SelectCharacterClassbyIndex (Variables|Default|GetLobbyGM_Ref) self 1))
    (:Out%202
      (Variables|Default|SetTeamID 1)
      (Default|SelectCharacterClassbyIndex (Variables|Default|GetLobbyGM_Ref) self 2)))
  (bind _asbp_our_game_instance (Utilities|Casting|CastToBP_OurGameInstance (Game|GetGameInstance)))
  (Default|SetTeamID _asbp_our_game_instance (Variables|Default|GetTeamID))
  (Development|PrintString (Utilities|String|ToString(Text) (Utilities|Text|FormatText "TeamID = {ID}" (Variables|Default|GetTeamID)))))

(event Custom|Ready
  (Development|PrintString "ready" true true "(R=0.000000,G=0.660000,B=1.000000,A=1.000000)" 1e+01)
  (CallFunction|ToggleReadyStatusonServer))

(event Custom|TryAgainUpdating
  (CallFunction|TryAgainUpdatingLobbyInfo))

(event EventBeginPlay
  (bind _asbp_lobby_gm (Utilities|Casting|CastToBP_LobbyGM (Game|GetGameMode)))
  (Variables|Default|SetLobbyGM_Ref _asbp_lobby_gm)
  (Variables|Default|SetbShowMouseCursor true)
  ;[1 1 1] 空のUI
  (bind _returnvalue (UserInterface|CreateWidget "/Game/Lobby/WB_GamePlayUI.WB_GamePlayUI_C" (Game|GetPlayerController 0)))
  (if (Utilities|IsValid _returnvalue)
    (bind _output_get (Variables|Default|SetGamePlayUI%20Ref _returnvalue))
    (UserInterface|Viewport|AddtoViewport _output_get 0)
    (Variables|Default|SetbShowMouseCursor true)
    (Input|SetInputModeGameandUI self 0 "DoNotLock" true false)
    (CallFunction|SetUp self)
    (Variables|Default|SetbShowMouseCursor true)
    (Input|SetInputModeUIOnly self 0 "DoNotLock" false)
    (Variables|Default|SetbShowMouseCursor false)
    (Input|SetInputModeGameOnly self false)
    (Development|PrintString "Hello" true true "(R=0.000000,G=0.660000,B=1.000000,A=1.000000)" 1e+01)
    (bind _aslobby_hud (Utilities|Casting|CastToLobbyHUD (HUD|GetHUD)))
    (bind _lobbyhud (Default|GetLobbyUI _aslobby_hud))
    (CallFunction|SetLobbyUI _lobbyhud)
    (else
      (Development|PrintString "プレイヤーUIが見つかりません。" true true "(R=1.000000,G=0.000000,B=0.013789,A=1.000000)" 1e+01))))

(event Input|KeyboardEvents|R
  (params (Key :type Key%20Structure))
  (:Pressed
    (CallFunction|Ready)))

(fn ConstructionScript)

(fn SetUp
  (if (Pawn|IsLocalPlayerController)
    (Variables|Default|SetbShowMouseCursor true)
    (Input|SetInputModeGameandUI self 0 "DoNotLock" false false)
    (CallFunction|SetPlayerNameonServer (Variables|/Game/Lobby/BP_OurGameInstance.BP_OurGameInstance_C|GetPlayerName (.AsBP%20Our%20Game%20Instance (Utilities|Casting|CastToBP_OurGameInstance (Game|GetGameInstance)))))))

(fn SetLobbyUI
  (params (lobbyUi :type WB%20Lobby%20UI%20Object%20Reference))
  (Variables|Default|SetLobbyUI_Ref lobbyUi))